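; UIPlayerController is a player controller for the main menu that creates the menu widget and relays navigation input to it.
; On BeginPlay it shows the mouse cursor, adds the widget to the viewport and focuses it in Game and UI input mode.
; That mode lets the left, right, up and down menu input actions reach the controller, which passes each to the widget's RechieveInputRequest as an enum value.
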(event EventBeginPlay
  (Variables|Default|SetbShowMouseCursor true)
  (bind _returnvalue (UserInterface|CreateWidget "/Game/_Game/Blueprints/MainMenuWidget.MainMenuWidget_C" (Game|GetPlayerController 0)))
  (bind _output_get (Variables|Default|SetMainMenuWidget_Ref _returnvalue))
  (UserInterface|Viewport|AddtoViewport _output_get 0)
  (Input|SetInputModeGameandUI (Game|GetPlayerController 0) (Variables|Default|GetMainMenuWidget_Ref) "DoNotLock" true))

(event Input|ActionEvents|InputActionMenuLeftNav
  (params (Key :type Key%20Structure))
  (:Pressed
    (Default|RechieveInputRequest (Variables|Default|GetMainMenuWidget_Ref) "NewEnumerator0")))

(event Input|ActionEvents|InputActionMenuRightNav
  (params (Key :type Key%20Structure))
  (:Pressed
    (Default|RechieveInputRequest (Variables|Default|GetMainMenuWidget_Ref) "NewEnumerator1")))

(event Input|ActionEvents|InputActionMenuUpNav
  (params (Key :type Key%20Structure))
  (:Pressed
    (Default|RechieveInputRequest (Variables|Default|GetMainMenuWidget_Ref) "NewEnumerator3")))

(event Input|ActionEvents|InputActionMenuDownNav
  (params (Key :type Key%20Structure))
  (:Pressed
    (Default|RechieveInputRequest (Variables|Default|GetMainMenuWidget_Ref) "NewEnumerator4")))

(fn ConstructionScript)