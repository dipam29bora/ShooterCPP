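; ArrowGirl is an archer character Blueprint that carries a bow, fires arrows and supports an aiming camera.
; On BeginPlay it caches its WarriorGirlAnimBP, binds that animation Blueprint's fire callback to release the current bow's arrow, and spawns a BP_SimpleBow attached to a keeping socket.
; AdjustCamera shortens and offsets the camera boom while aiming.
; Leftover radar and arrow-spawn nodes never run.
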(event Custom|FireArrow
  (Class|BowActor|ReleaseArrow (Variables|Default|GetcurrentBow)))

(event EventBeginPlay
  (|CallParentFunction)
  (Utilities|FlowControl|Sequence
    (:then_0
      (bind _aswarrior_girl_anim_bp (Utilities|Casting|CastToWarriorGirlAnimBP (Components|SkeletalMesh|GetAnimInstance (Variables|Character|GetMesh))))
      (Variables|Default|SetAnimBP _aswarrior_girl_anim_bp))
    (:then_1
      (EventDispatchers|BindEventtoFireArrowCallback (Variables|Default|GetAnimBP) (delegate Custom|FireArrow)))
    (:then_2
      (bind _returnvalue (Game|SpawnActorfromClass "/Game/Blueprints/Weapons/BP_SimpleBow.BP_SimpleBow_C" (Transformation|GetSocketTransform (Variables|Character|GetMesh) "BowKeepingSocket" "RTS_World") "Undefined" 0 0))
      (Class|ArrowGirlCharacter|SetCurrentBow _returnvalue)
      (Transformation|AttachComponentToComponent (Class|ArrowGirlCharacter|GetCurrentBow) (Variables|Character|GetMesh) "BowKeepingSocket" "SnapToTarget" "SnapToTarget" "KeepRelative" true))))

(event EventAdjustCamera
  (bind _returnvalue (Class|ArrowGirlCharacter|GetCameraBoom))
  (if (Variables|Default|GetIsAiming)
    (Variables|/Script/Engine.SpringArmComponent|SetTargetArmLength _returnvalue 2e+02)
    (Variables|/Script/Engine.SpringArmComponent|SetSocketOffset _returnvalue "0,-60.000000, 0")
    (else
      (Variables|/Script/Engine.SpringArmComponent|SetTargetArmLength _returnvalue 4e+02)
      (Variables|/Script/Engine.SpringArmComponent|SetSocketOffset _returnvalue "0, 0, 0"))))

(fn ConstructionScript)