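; Arrow_BP is an arrow projectile actor for the weapons system.
; On BeginPlay it sets the projectile movement component's initial and max speed from its ForceFector variable.
; Each tick, FacingTowardsDirection pitches the arrow to match its velocity vector while keeping its current roll and yaw, so the tip follows the flight arc.
; The overlap event is empty, so no hit handling happens here.
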(event EventBeginPlay
  (bind _projectilemovement (Variables|Default|GetProjectileMovement))
  (bind _forcefector (Variables|Default|GetForceFector))
  (Variables|/Script/Engine.ProjectileMovementComponent|SetInitialSpeed _projectilemovement _forcefector)
  (Variables|/Script/Engine.ProjectileMovementComponent|SetMaxSpeed _projectilemovement _forcefector))

(event Collision|EventActorBeginOverlap
  (params (OtherActor :type Actor%20Object%20Reference)))

(event EventTick
  (params (DeltaSeconds :type Float%20%28single-precision%29))
  (CallFunction|FacingTowardsDirection))

(fn ConstructionScript)

(fn FacingTowardsDirection
  (bind _returnvalue (Transformation|GetActorRotation))
  (bind (_roll _pitch _yaw) (Math|Rotator|BreakRotator _returnvalue))
  (Transformation|SetActorRotation (Math|Rotator|MakeRotator _roll (.Pitch (Math|Rotator|BreakRotator (Math|Rotator|MakeRotfromX (Transformation|GetVelocity)))) _yaw)))