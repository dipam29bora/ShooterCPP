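; MovingActor is an actor that moves its Cube component along world X when play begins.
; A timeline plays from the start, and each update adds its MoveAlpha, scaled by NewVar0, to the cube's current X without sweeping.
; The offset therefore accumulates per update rather than interpolating between fixed endpoints.
; When the timeline finishes, the NewVar1 flag decides whether a timeline Reverse is called.
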(event EventBeginPlay
  (bind _cube (Variables|Default|GetCube))
  (bind _returnvalue (Transformation|GetWorldLocation _cube))
  (bind (_x _y _z) (Math|Vector|BreakVector _returnvalue))
  (bind _movealpha (Timeline|Timeline_0 PlayFromStart)
    (:Update
      (Transformation|SetWorldLocation _cube (Math|Vector|MakeVector (+ _x (* _movealpha (Variables|Default|GetNewVar_0))) _y _z) false false))
    (:Finished
      (if (Variables|Default|GetNewVar_1)
        (Utilities|String|Reverse (Variables|Default|GetTimeline_0))))))

(event Collision|EventActorBeginOverlap
  (params (OtherActor :type Actor%20Object%20Reference)))

(event EventTick
  (params (DeltaSeconds :type Float%20%28single-precision%29)))

(fn ConstructionScript)