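; Behavior tree task that has an AI pawn, filed under deer AI, eat at a food point along its patrol path.
; Each tick it uses the blackboard index to fetch the FoodPoints entry from the pawn's PatrollingPathComponent, flagging it as being eaten while food is not negative.
; Once the amount drops below zero, the task finishes successfully and resets that food point.
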(event EventReceiveTickAI
  (params (OwnerController :type AI%20Controller%20Object%20Reference) (ControlledPawn :type Pawn%20Object%20Reference) (DeltaSeconds :type Float%20%28single-precision%29))
  (bind _asfood_points (Utilities|Casting|CastToFoodPoints (Utilities|Array|Get(acopy) (Variables|/Script/ShooterCPP.PatrollingPathComponent|GetPatrolPointsForBP (Actor|GetComponentbyClass ControlledPawn "/Script/ShooterCPP.PatrollingPathComponent")) (Class|BTFunctionLibrary|GetBlackboardValueasInt (Variables|Default|GetIndexKey)))))
  (if (>= (Variables|/Script/ShooterCPP.FoodPoints|GetFoodAmount _asfood_points) 0.0)
    (Variables|/Script/ShooterCPP.FoodPoints|SetIsEating _asfood_points true)
    (else
      (AI|BehaviorTree|FinishExecute true)
      (Class|FoodPoints|ResetFoodPoint _asfood_points))))